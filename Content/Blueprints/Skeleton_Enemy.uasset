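; Skeleton enemy character with a flipbook sprite that turns toward the player and moves until within a fixed horizontal range.
; Each Tick yaws it toward the player, picks the walk flipbook when moving or the attack one when still, then updates movement.
; Movement feeds the player's world position in as the input direction, signed by relative X, and zeroes velocity in range.
; The attack is animation only, with no damage logic.
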(event Custom|AnimationUpdate
  (Sprite|SetFlipbook (Variables|Default|GetSprite) (select (> (Math|Vector|VectorLength (Variables|/Script/Engine.MovementComponent|GetVelocity (Variables|Character|GetCharacterMovement))) 0.0) (Variables|Default|GetSkele_Walk) (Variables|Default|GetSkele_Attack))))

(event Custom|MovementUpdate
  (bind _returnvalue (Game|GetPlayerCharacter 0))
  (bind _returnvalue_2 (Game|GetPlayerCharacter 0))
  (bind _returnvalue_3 (Transformation|GetActorLocation _returnvalue))
  (bind _returnvalue_4 (Transformation|GetActorLocation _returnvalue_2))
  (bind (_x _y _z) (Math|Vector|BreakVector _returnvalue_3))
  (bind (_x_2 _y_2 _z_2) (Math|Vector|BreakVector _returnvalue_4))
  (if (> (Transformation|GetHorizontalDistanceTo (Game|GetPlayerCharacter 0)) 2e+02)
    (if (< (.X (Math|Vector|BreakVector (Math|Vector|GetUnitDirection(Vector) (Transformation|GetActorLocation (Game|GetPlayerCharacter 0)) (Transformation|GetActorLocation)))) 0.0)
      (Pawn|Input|AddMovementInput (Math|Vector|MakeVector _x_2 _y_2 _z_2) 0.1 false)
      (else
        (Pawn|Input|AddMovementInput (Math|Vector|MakeVector _x _y _z) -0.1 false)))
    (else
      (Variables|/Script/Engine.MovementComponent|SetVelocity (Variables|Character|GetCharacterMovement) "0, 0, 0"))))

(event EventBeginPlay)

(event EventTick
  (params (DeltaSeconds :type Float%20%28single-precision%29))
  (Transformation|SetActorRotation (Math|Rotator|FindLookatRotation (* (Transformation|GetActorLocation) "1.000000,1.000000,0.000000") (* (Transformation|GetActorLocation (Game|GetPlayerCharacter 0)) "1.000000,1.000000,0.000000")))
  (CallFunction|AnimationUpdate)
  (CallFunction|MovementUpdate))

(fn ConstructionScript)

(fn GetUnitVector)